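; Procedural level generator that lays out connected floor rooms on a grid at BeginPlay and fits each with walls.
; A random walk from the start room records positions in RoomLocation, continuing in the same direction past occupied cells until it finds a free one.
; A second pass checks each room's four neighbours against that array and spawns the wall Blueprint matching its exit combination.
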(event EventBeginPlay
  (Utilities|FlowControl|Sequence
    (:then_0
      (CallFunction|Initialise))
    (:then_1
      (Game|SpawnActorfromClass "/Game/Level/Exits/BP_Floor.BP_Floor_C" (Math|Transform|MakeTransform (Variables|Default|GetSTART_ROOM_POSITION) (Variables|Default|GetTILEMAP_TRANSFORM_ROTATION) "1,1,1") "Undefined" 0 0))
    (:then_2
      (Utilities|Array|SetArrayElem (Variables|Default|GetroomLocation) (Variables|Default|GetSTART_ROOM_NUMBER) (Variables|Default|GetmainRoomPosition)))
    (:then_3
      (for _index (range (Variables|Default|GetFIRST_ROOM_NUMBER) (Variables|Default|GetNUMBER_OF_ROOMS))
        (Variables|Default|SetroomNumber _index)
        (Utilities|FlowControl|Sequence :!label _label
          (:then_0
            (if (not (Variables|Default|GetroomCreated))
              (CallFunction|GetRandomDirection)))
          (:then_1
            (CallFunction|SetNewRoomGeneratorPoint))
          (:then_2
            (Variables|Default|SetroomCreated false))
          (:then_3
            (CallFunction|CheckValidRoomLocation (Variables|Default|GetmainRoomPosition)))
          (:then_4
            (if (Variables|Default|GetroomCreated)
              (goto _label)
              (else
                (CallFunction|GenerateRoom))))))
      (Utilities|FlowControl|Sequence
        (:then_0
          (CallFunction|CreateWalls (Variables|Default|GetSTART_ROOM_POSITION)))
        (:then_1
          (for _index_2 (range (Variables|Default|GetSTART_ROOM_NUMBER) (Variables|Default|GetNUMBER_OF_ROOMS))
            (CallFunction|CreateWalls (Utilities|Array|Get(acopy) (Variables|Default|GetroomLocation) _index_2))))
        (:then_2
          (CallFunction|CreateWalls (Variables|Default|GetendRoomPosition)))))))

(fn ConstructionScript)

(fn SetNewRoomGeneratorPoint
  (if (== (Variables|Default|GetselectedDirection) (Variables|Default|GetNORTH))
    (Variables|Default|SetmainRoomPosition (Math|Vector|MakeVector (.x (Variables|Default|GetmainRoomPosition)) (+ (.y (Variables|Default|GetmainRoomPosition)) (Variables|Default|GetROOM_OFFSET_POSITION_Y)) 0.0))
    (elif (== (Variables|Default|GetselectedDirection) (Variables|Default|GetSOUTH))
      (Variables|Default|SetmainRoomPosition (Math|Vector|MakeVector (.x (Variables|Default|GetmainRoomPosition)) (+ (.y (Variables|Default|GetmainRoomPosition)) (* -1 (Variables|Default|GetROOM_OFFSET_POSITION_Y))) 0.0))
      (elif (== (Variables|Default|GetselectedDirection) (Variables|Default|GetWEST))
        (Variables|Default|SetmainRoomPosition (Math|Vector|MakeVector (+ (.x (Variables|Default|GetmainRoomPosition)) (* -1 (Variables|Default|GetROOM_OFFSET_POSITION_X))) (.y (Variables|Default|GetmainRoomPosition)) 0.0))
        (elif (== (Variables|Default|GetselectedDirection) (Variables|Default|GetEAST))
          (Variables|Default|SetmainRoomPosition (Math|Vector|MakeVector (+ (.x (Variables|Default|GetmainRoomPosition)) (Variables|Default|GetROOM_OFFSET_POSITION_X)) (.y (Variables|Default|GetmainRoomPosition)) 0.0)))))))

(fn GetRandomDirection
  (Variables|Default|SetselectedDirection (Math|Random|RandomIntegerinRange 0 (- (Variables|Default|GetNUMBER_OF_DIRECTIONS) 1))))

(fn GenerateRoom
  (Utilities|FlowControl|Sequence
    (:then_0
      (if (== (Variables|Default|GetroomNumber) (Variables|Default|GetNUMBER_OF_ROOMS))
        (Game|SpawnActorfromClass "/Game/Level/Exits/BP_Floor.BP_Floor_C" (Math|Transform|MakeTransform (Variables|Default|GetmainRoomPosition) (Variables|Default|GetTILEMAP_TRANSFORM_ROTATION) "1,1,1") "Undefined" 0 0)
        (else
          (Game|SpawnActorfromClass "/Game/Level/Exits/BP_Floor.BP_Floor_C" (Math|Transform|MakeTransform (Variables|Default|GetmainRoomPosition) (Variables|Default|GetTILEMAP_TRANSFORM_ROTATION) "1,1,1") "Undefined" 0 0))))
    (:then_1
      (Utilities|Array|SetArrayElem (Variables|Default|GetroomLocation) (Variables|Default|GetroomNumber) (Variables|Default|GetmainRoomPosition)))
    (:then_2
      (if (== (Variables|Default|GetroomNumber) (Variables|Default|GetNUMBER_OF_ROOMS))
        (Variables|Default|SetendRoomPosition (Variables|Default|GetmainRoomPosition))))))

(fn Initialise
  (for _index (range (Variables|Default|GetSTART_ROOM_NUMBER) (Variables|Default|GetNUMBER_OF_ROOMS))
    (Utilities|Array|Add (Variables|Default|GetroomLocation) (Math|Vector|MakeVector 0.0 0.0 0.0))))

(fn CheckValidRoomLocation
  (params (roomPosition :type Vector))
  (for _index (range (Variables|Default|GetSTART_ROOM_NUMBER) (Variables|Default|GetNUMBER_OF_ROOMS))
    (if (Math|Vector|Equal(Vector) (Utilities|Array|Get(acopy) (Variables|Default|GetroomLocation) _index) roomPosition 0.0001)
      (Variables|Default|SetroomCreated true))))

(fn CreateWalls
  (params (roomPositionVector :type Vector))
  (Variables|Default|SetcurrentRoom roomPositionVector)
  (Utilities|FlowControl|Sequence
    (:then_0
      (LocalVariables|SetavailableExits 0))
    (:then_1
      (LocalVariables|SetisNorthExit (Math|Vector|MakeVector (.x (Variables|Default|GetcurrentRoom)) (- (.y (Variables|Default|GetcurrentRoom)) (Variables|Default|GetROOM_OFFSET_POSITION_Y)) 0.0))
      (Variables|Default|SetroomCreated false)
      (Variables|Default|SethasNorthExit false)
      (CallFunction|CheckValidRoomLocation (LocalVariables|GetisNorthExit))
      (if (Variables|Default|GetroomCreated)
        (LocalVariables|SetavailableExits (+ (LocalVariables|GetavailableExits) 1))
        (Variables|Default|SethasNorthExit true)))
    (:then_2
      (LocalVariables|SetisEastExit (Math|Vector|MakeVector (+ (.x (Variables|Default|GetcurrentRoom)) (Variables|Default|GetROOM_OFFSET_POSITION_X)) (.y (Variables|Default|GetcurrentRoom)) 0.0))
      (Variables|Default|SetroomCreated false)
      (Variables|Default|SethasEastExit false)
      (CallFunction|CheckValidRoomLocation (LocalVariables|GetisEastExit))
      (if (Variables|Default|GetroomCreated)
        (LocalVariables|SetavailableExits (+ (LocalVariables|GetavailableExits) 1))
        (Variables|Default|SethasEastExit true)))
    (:then_3
      (LocalVariables|SetisSouthExit (Math|Vector|MakeVector (.x (Variables|Default|GetcurrentRoom)) (+ (.y (Variables|Default|GetcurrentRoom)) (Variables|Default|GetROOM_OFFSET_POSITION_Y)) 0.0))
      (Variables|Default|SetroomCreated false)
      (Variables|Default|SethasSouthExit false)
      (CallFunction|CheckValidRoomLocation (LocalVariables|GetisSouthExit))
      (if (Variables|Default|GetroomCreated)
        (LocalVariables|SetavailableExits (+ (LocalVariables|GetavailableExits) 1))
        (Variables|Default|SethasSouthExit true)))
    (:then_4
      (LocalVariables|SetisWestExit (Math|Vector|MakeVector (- (.x (Variables|Default|GetcurrentRoom)) (Variables|Default|GetROOM_OFFSET_POSITION_X)) (.y (Variables|Default|GetcurrentRoom)) 0.0))
      (Variables|Default|SetroomCreated false)
      (Variables|Default|SethasWestExit false)
      (CallFunction|CheckValidRoomLocation (LocalVariables|GetisWestExit))
      (if (Variables|Default|GetroomCreated)
        (LocalVariables|SetavailableExits (+ (LocalVariables|GetavailableExits) 1))
        (Variables|Default|SethasWestExit true)))
    (:then_5
      (if (== (LocalVariables|GetavailableExits) 1)
        (CallFunction|OneExit)
        (elif (== (LocalVariables|GetavailableExits) 2)
          (CallFunction|TwoExits)
          (elif (== (LocalVariables|GetavailableExits) 3)
            (CallFunction|ThreeExits)
            (elif (== (LocalVariables|GetavailableExits) 4)
              (CallFunction|FourExits))))))))

(fn OneExit
  (if (Variables|Default|GethasNorthExit)
    (Game|SpawnActorfromClass "/Game/Level/Exits/BP_N.BP_N_C" (Math|Transform|MakeTransform (Variables|Default|GetcurrentRoom) (Variables|Default|GetTILEMAP_TRANSFORM_ROTATION) "1,1,1") "Undefined" 0 0)
    (elif (Variables|Default|GethasEastExit)
      (Game|SpawnActorfromClass "/Game/Level/Exits/BP_E.BP_E_C" (Math|Transform|MakeTransform (Variables|Default|GetcurrentRoom) (Variables|Default|GetTILEMAP_TRANSFORM_ROTATION) "1,1,1") "Undefined" 0 0)
      (elif (Variables|Default|GethasSouthExit)
        (Game|SpawnActorfromClass "/Game/Level/Exits/BP_S.BP_S_C" (Math|Transform|MakeTransform (Variables|Default|GetcurrentRoom) (Variables|Default|GetTILEMAP_TRANSFORM_ROTATION) "1,1,1") "Undefined" 0 0)
        (elif (Variables|Default|GethasWestExit)
          (Game|SpawnActorfromClass "/Game/Level/Exits/BP_W.BP_W_C" (Math|Transform|MakeTransform (Variables|Default|GetcurrentRoom) (Variables|Default|GetTILEMAP_TRANSFORM_ROTATION) "1,1,1") "Undefined" 0 0))))))

(fn TwoExits
  (if (and (Variables|Default|GethasNorthExit) (Variables|Default|GethasSouthExit))
    (Game|SpawnActorfromClass "/Game/Level/Exits/BP_NS.BP_NS_C" (Math|Transform|MakeTransform (Variables|Default|GetcurrentRoom) (Variables|Default|GetTILEMAP_TRANSFORM_ROTATION) "1,1,1") "Undefined" 0 0)
    (elif (and (Variables|Default|GethasEastExit) (Variables|Default|GethasWestExit))
      (Game|SpawnActorfromClass "/Game/Level/Exits/BP_EW.BP_EW_C" (Math|Transform|MakeTransform (Variables|Default|GetcurrentRoom) (Variables|Default|GetTILEMAP_TRANSFORM_ROTATION) "1,1,1") "Undefined" 0 0)
      (elif (and (Variables|Default|GethasNorthExit) (Variables|Default|GethasEastExit))
        (Game|SpawnActorfromClass "/Game/Level/Exits/BP_NE.BP_NE_C" (Math|Transform|MakeTransform (Variables|Default|GetcurrentRoom) (Variables|Default|GetTILEMAP_TRANSFORM_ROTATION) "1,1,1") "Undefined" 0 0)
        (elif (and (Variables|Default|GethasEastExit) (Variables|Default|GethasSouthExit))
          (Game|SpawnActorfromClass "/Game/Level/Exits/BP_SE.BP_SE_C" (Math|Transform|MakeTransform (Variables|Default|GetcurrentRoom) (Variables|Default|GetTILEMAP_TRANSFORM_ROTATION) "1,1,1") "Undefined" 0 0)
          (elif (and (Variables|Default|GethasNorthExit) (Variables|Default|GethasWestExit))
            (Game|SpawnActorfromClass "/Game/Level/Exits/BP_NW.BP_NW_C" (Math|Transform|MakeTransform (Variables|Default|GetcurrentRoom) (Variables|Default|GetTILEMAP_TRANSFORM_ROTATION) "1,1,1") "Undefined" 0 0)
            (elif (and (Variables|Default|GethasSouthExit) (Variables|Default|GethasWestExit))
              (Game|SpawnActorfromClass "/Game/Level/Exits/BP_SW.BP_SW_C" (Math|Transform|MakeTransform (Variables|Default|GetcurrentRoom) (Variables|Default|GetTILEMAP_TRANSFORM_ROTATION) "1,1,1") "Undefined" 0 0))))))))

(fn ThreeExits
  (if (Math|Boolean|ANDBoolean (Variables|Default|GethasNorthExit) (Variables|Default|GethasEastExit) (Variables|Default|GethasSouthExit))
    (Game|SpawnActorfromClass "/Game/Level/Exits/BP_NSE.BP_NSE_C" (Math|Transform|MakeTransform (Variables|Default|GetcurrentRoom) (Variables|Default|GetTILEMAP_TRANSFORM_ROTATION) "1,1,1") "Undefined" 0 0)
    (elif (Math|Boolean|ANDBoolean (Variables|Default|GethasNorthExit) (Variables|Default|GethasWestExit) (Variables|Default|GethasSouthExit))
      (Game|SpawnActorfromClass "/Game/Level/Exits/BP_NSW.BP_NSW_C" (Math|Transform|MakeTransform (Variables|Default|GetcurrentRoom) (Variables|Default|GetTILEMAP_TRANSFORM_ROTATION) "1,1,1") "Undefined" 0 0)
      (elif (Math|Boolean|ANDBoolean (Variables|Default|GethasNorthExit) (Variables|Default|GethasEastExit) (Variables|Default|GethasWestExit))
        (Game|SpawnActorfromClass "/Game/Level/Exits/BP_NEW.BP_NEW_C" (Math|Transform|MakeTransform (Variables|Default|GetcurrentRoom) (Variables|Default|GetTILEMAP_TRANSFORM_ROTATION) "1,1,1") "Undefined" 0 0)
        (elif (Math|Boolean|ANDBoolean (Variables|Default|GethasSouthExit) (Variables|Default|GethasEastExit) (Variables|Default|GethasWestExit))
          (Game|SpawnActorfromClass "/Game/Level/Exits/BP_SEW.BP_SEW_C" (Math|Transform|MakeTransform (Variables|Default|GetcurrentRoom) (Variables|Default|GetTILEMAP_TRANSFORM_ROTATION) "1,1,1") "Undefined" 0 0))))))

(fn FourExits
  (if (Math|Boolean|ANDBoolean (Variables|Default|GethasNorthExit) (Variables|Default|GethasEastExit) (Variables|Default|GethasSouthExit) (Variables|Default|GethasWestExit))
    (Game|SpawnActorfromClass "/Game/Level/Exits/BP_NESW.BP_NESW_C" (Math|Transform|MakeTransform (Variables|Default|GetcurrentRoom) (Variables|Default|GetTILEMAP_TRANSFORM_ROTATION) "1,1,1") "Undefined" 0 0)))