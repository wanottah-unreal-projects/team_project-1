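; Level exit piece with north, east, south and west sliding double doors that open for a TwinStickPawn.
; Each door controller's overlap opens its pair or closes it after a one-second delay on exit.
; Timelines lerp panels from their current location to targets offset by TILESIZE along relative X, despite East/West variables named Y.
; West closing never sets WestLeftClosedDoorPosition, writing WestRightClosedDoorPosition twice instead.
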(event OnComponentBeginOverlap(NorthDoorController)
  (params (OverlappedComponent :type Primitive%20Component%20Object%20Reference) (OtherActor :type Actor%20Object%20Reference) (OtherComp :type Primitive%20Component%20Object%20Reference) (OtherBodyIndex :type Integer) (bFromSweep :type Boolean) (SweepResult :type Hit%20Result%20Structure%20%28by%20ref%29))
  (bind _north_door_right (Variables|Default|GetNorth_Door_Right))
  (bind _north_door_right_2 (Variables|Default|GetNorth_Door_Right))
  (bind _north_door_left (Variables|Default|GetNorth_Door_Left))
  (bind _north_door_left_2 (Variables|Default|GetNorth_Door_Left))
  (bind _relativelocation (Variables|/Script/Engine.SceneComponent|GetRelativeLocation _north_door_right))
  (bind _relativelocation_2 (Variables|/Script/Engine.SceneComponent|GetRelativeLocation _north_door_left))
  (bind _relativelocation_3 (Variables|/Script/Engine.SceneComponent|GetRelativeLocation _north_door_left_2))
  (bind _relativelocation_4 (Variables|/Script/Engine.SceneComponent|GetRelativeLocation _north_door_right_2))
  (Utilities|Casting|CastToTwinStickPawn OtherActor)
  (Variables|Default|SetopenNorthDoor true)
  (if (Variables|Default|GetopenNorthDoor)
    (Variables|Default|SetnorthRelativeLeftDoorLocationX (- (.x _relativelocation_2) (Variables|Default|GetTILE_SIZE)))
    (Variables|Default|SetnorthLeftOpenDoorPosition (Math|Vector|MakeVector (Variables|Default|GetnorthRelativeLeftDoorLocationX) (.y _relativelocation_2) (.z _relativelocation_2)))
    (Variables|Default|SetnorthRelativeRightDoorLocationX (+ (Variables|Default|GetTILE_SIZE) (.x _relativelocation_4)))
    (Variables|Default|SetnorthRightOpenDoorPosition (Math|Vector|MakeVector (Variables|Default|GetnorthRelativeRightDoorLocationX) (.y _relativelocation_4) (.z _relativelocation_4)))
    (bind _opendoor (Timeline|Timeline_0 PlayFromStart)
      (:Update
        (Transformation|SetRelativeLocation (Variables|Default|GetNorth_Door_Left) (Math|Vector|Lerp(Vector) (Variables|/Script/Engine.SceneComponent|GetRelativeLocation (Variables|Default|GetNorth_Door_Left)) (Variables|Default|GetnorthLeftOpenDoorPosition) _opendoor) false false)
        (Transformation|SetRelativeLocation (Variables|Default|GetNorth_Door_Right) (Math|Vector|Lerp(Vector) (Variables|/Script/Engine.SceneComponent|GetRelativeLocation (Variables|Default|GetNorth_Door_Right)) (Variables|Default|GetnorthRightOpenDoorPosition) _opendoor) false false)))
    (else
      (Utilities|FlowControl|Delay 1.0)
      (Variables|Default|SetnorthRelativeLeftDoorLocationX (+ (Variables|Default|GetTILE_SIZE) (.x _relativelocation_3)))
      (Variables|Default|SetnorthLeftClosedDoorPosition (Math|Vector|MakeVector (Variables|Default|GetnorthRelativeLeftDoorLocationX) (.y _relativelocation_3) (.z _relativelocation_3)))
      (Variables|Default|SetnorthRelativeRightDoorLocationX (- (.x _relativelocation) (Variables|Default|GetTILE_SIZE)))
      (Variables|Default|SetnorthRightClosedDoorPosition (Math|Vector|MakeVector (Variables|Default|GetnorthRelativeRightDoorLocationX) (.y _relativelocation) (.z _relativelocation)))
      (bind _closedoor (Timeline|Timeline_1 PlayFromStart)
        (:Update
          (Transformation|SetRelativeLocation (Variables|Default|GetNorth_Door_Left) (Math|Vector|Lerp(Vector) (Variables|/Script/Engine.SceneComponent|GetRelativeLocation (Variables|Default|GetNorth_Door_Left)) (Variables|Default|GetnorthLeftClosedDoorPosition) _closedoor) false false)
          (Transformation|SetRelativeLocation (Variables|Default|GetNorth_Door_Right) (Math|Vector|Lerp(Vector) (Variables|/Script/Engine.SceneComponent|GetRelativeLocation (Variables|Default|GetNorth_Door_Right)) (Variables|Default|GetnorthRightClosedDoorPosition) _closedoor) false false))))))

(event OnComponentBeginOverlap(EastDoorController)
  (params (OverlappedComponent :type Primitive%20Component%20Object%20Reference) (OtherActor :type Actor%20Object%20Reference) (OtherComp :type Primitive%20Component%20Object%20Reference) (OtherBodyIndex :type Integer) (bFromSweep :type Boolean) (SweepResult :type Hit%20Result%20Structure%20%28by%20ref%29))
  (bind _east_door_left (Variables|Default|GetEast_Door_Left))
  (bind _east_door_right (Variables|Default|GetEast_Door_Right))
  (bind _east_door_right_2 (Variables|Default|GetEast_Door_Right))
  (bind _east_door_left_2 (Variables|Default|GetEast_Door_Left))
  (bind _relativelocation (Variables|/Script/Engine.SceneComponent|GetRelativeLocation _east_door_right_2))
  (bind _relativelocation_2 (Variables|/Script/Engine.SceneComponent|GetRelativeLocation _east_door_right))
  (bind _relativelocation_3 (Variables|/Script/Engine.SceneComponent|GetRelativeLocation _east_door_left_2))
  (bind _relativelocation_4 (Variables|/Script/Engine.SceneComponent|GetRelativeLocation _east_door_left))
  (Utilities|Casting|CastToTwinStickPawn OtherActor)
  (Variables|Default|SetopenEastDoor true)
  (if (Variables|Default|GetopenEastDoor)
    (Variables|Default|SeteastRelativeLeftDoorLocationY (- (.x _relativelocation_3) (Variables|Default|GetTILE_SIZE)))
    (Variables|Default|SeteastLeftOpenDoorPosition (Math|Vector|MakeVector (Variables|Default|GeteastRelativeLeftDoorLocationY) (.y _relativelocation_3) (.z _relativelocation_3)))
    (Variables|Default|SeteastRelativeRightDoorLocationY (+ (Variables|Default|GetTILE_SIZE) (.x _relativelocation)))
    (Variables|Default|SeteastRightOpenDoorPosition (Math|Vector|MakeVector (Variables|Default|GeteastRelativeRightDoorLocationY) (.y _relativelocation) (.z _relativelocation)))
    (bind _opendoor (Timeline|Timeline_2 PlayFromStart)
      (:Update
        (Transformation|SetRelativeLocation (Variables|Default|GetEast_Door_Left) (Math|Vector|Lerp(Vector) (Variables|/Script/Engine.SceneComponent|GetRelativeLocation (Variables|Default|GetEast_Door_Left)) (Variables|Default|GeteastLeftOpenDoorPosition) _opendoor) false false)
        (Transformation|SetRelativeLocation (Variables|Default|GetEast_Door_Right) (Math|Vector|Lerp(Vector) (Variables|/Script/Engine.SceneComponent|GetRelativeLocation (Variables|Default|GetEast_Door_Right)) (Variables|Default|GeteastRightOpenDoorPosition) _opendoor) false false)))
    (else
      (Utilities|FlowControl|Delay 1.0)
      (Variables|Default|SeteastRelativeLeftDoorLocationY (+ (Variables|Default|GetTILE_SIZE) (.x _relativelocation_4)))
      (Variables|Default|SeteastLeftClosedDoorPosition (Math|Vector|MakeVector (Variables|Default|GeteastRelativeLeftDoorLocationY) (.y _relativelocation_4) (.z _relativelocation_4)))
      (Variables|Default|SeteastRelativeRightDoorLocationY (- (.x _relativelocation_2) (Variables|Default|GetTILE_SIZE)))
      (Variables|Default|SeteastRightClosedDoorPosition (Math|Vector|MakeVector (Variables|Default|GeteastRelativeRightDoorLocationY) (.y _relativelocation_2) (.z _relativelocation_2)))
      (bind _closedoor (Timeline|Timeline_3 PlayFromStart)
        (:Update
          (Transformation|SetRelativeLocation (Variables|Default|GetEast_Door_Left) (Math|Vector|Lerp(Vector) (Variables|/Script/Engine.SceneComponent|GetRelativeLocation (Variables|Default|GetEast_Door_Left)) (Variables|Default|GeteastLeftClosedDoorPosition) _closedoor) false false)
          (Transformation|SetRelativeLocation (Variables|Default|GetEast_Door_Right) (Math|Vector|Lerp(Vector) (Variables|/Script/Engine.SceneComponent|GetRelativeLocation (Variables|Default|GetEast_Door_Right)) (Variables|Default|GeteastRightClosedDoorPosition) _closedoor) false false))))))

(event OnComponentEndOverlap(NorthDoorController)
  (params (OverlappedComponent :type Primitive%20Component%20Object%20Reference) (OtherActor :type Actor%20Object%20Reference) (OtherComp :type Primitive%20Component%20Object%20Reference) (OtherBodyIndex :type Integer))
  (bind _north_door_right (Variables|Default|GetNorth_Door_Right))
  (bind _north_door_right_2 (Variables|Default|GetNorth_Door_Right))
  (bind _north_door_left (Variables|Default|GetNorth_Door_Left))
  (bind _north_door_left_2 (Variables|Default|GetNorth_Door_Left))
  (bind _relativelocation (Variables|/Script/Engine.SceneComponent|GetRelativeLocation _north_door_right))
  (bind _relativelocation_2 (Variables|/Script/Engine.SceneComponent|GetRelativeLocation _north_door_left))
  (bind _relativelocation_3 (Variables|/Script/Engine.SceneComponent|GetRelativeLocation _north_door_left_2))
  (bind _relativelocation_4 (Variables|/Script/Engine.SceneComponent|GetRelativeLocation _north_door_right_2))
  (Utilities|Casting|CastToTwinStickPawn OtherActor)
  (Variables|Default|SetopenNorthDoor false)
  (if (Variables|Default|GetopenNorthDoor)
    (Variables|Default|SetnorthRelativeLeftDoorLocationX (- (.x _relativelocation_2) (Variables|Default|GetTILE_SIZE)))
    (Variables|Default|SetnorthLeftOpenDoorPosition (Math|Vector|MakeVector (Variables|Default|GetnorthRelativeLeftDoorLocationX) (.y _relativelocation_2) (.z _relativelocation_2)))
    (Variables|Default|SetnorthRelativeRightDoorLocationX (+ (Variables|Default|GetTILE_SIZE) (.x _relativelocation_4)))
    (Variables|Default|SetnorthRightOpenDoorPosition (Math|Vector|MakeVector (Variables|Default|GetnorthRelativeRightDoorLocationX) (.y _relativelocation_4) (.z _relativelocation_4)))
    (bind _opendoor (Timeline|Timeline_0 PlayFromStart)
      (:Update
        (Transformation|SetRelativeLocation (Variables|Default|GetNorth_Door_Left) (Math|Vector|Lerp(Vector) (Variables|/Script/Engine.SceneComponent|GetRelativeLocation (Variables|Default|GetNorth_Door_Left)) (Variables|Default|GetnorthLeftOpenDoorPosition) _opendoor) false false)
        (Transformation|SetRelativeLocation (Variables|Default|GetNorth_Door_Right) (Math|Vector|Lerp(Vector) (Variables|/Script/Engine.SceneComponent|GetRelativeLocation (Variables|Default|GetNorth_Door_Right)) (Variables|Default|GetnorthRightOpenDoorPosition) _opendoor) false false)))
    (else
      (Utilities|FlowControl|Delay 1.0)
      (Variables|Default|SetnorthRelativeLeftDoorLocationX (+ (Variables|Default|GetTILE_SIZE) (.x _relativelocation_3)))
      (Variables|Default|SetnorthLeftClosedDoorPosition (Math|Vector|MakeVector (Variables|Default|GetnorthRelativeLeftDoorLocationX) (.y _relativelocation_3) (.z _relativelocation_3)))
      (Variables|Default|SetnorthRelativeRightDoorLocationX (- (.x _relativelocation) (Variables|Default|GetTILE_SIZE)))
      (Variables|Default|SetnorthRightClosedDoorPosition (Math|Vector|MakeVector (Variables|Default|GetnorthRelativeRightDoorLocationX) (.y _relativelocation) (.z _relativelocation)))
      (bind _closedoor (Timeline|Timeline_1 PlayFromStart)
        (:Update
          (Transformation|SetRelativeLocation (Variables|Default|GetNorth_Door_Left) (Math|Vector|Lerp(Vector) (Variables|/Script/Engine.SceneComponent|GetRelativeLocation (Variables|Default|GetNorth_Door_Left)) (Variables|Default|GetnorthLeftClosedDoorPosition) _closedoor) false false)
          (Transformation|SetRelativeLocation (Variables|Default|GetNorth_Door_Right) (Math|Vector|Lerp(Vector) (Variables|/Script/Engine.SceneComponent|GetRelativeLocation (Variables|Default|GetNorth_Door_Right)) (Variables|Default|GetnorthRightClosedDoorPosition) _closedoor) false false))))))

(event OnComponentEndOverlap(EastDoorController)
  (params (OverlappedComponent :type Primitive%20Component%20Object%20Reference) (OtherActor :type Actor%20Object%20Reference) (OtherComp :type Primitive%20Component%20Object%20Reference) (OtherBodyIndex :type Integer))
  (bind _east_door_left (Variables|Default|GetEast_Door_Left))
  (bind _east_door_right (Variables|Default|GetEast_Door_Right))
  (bind _east_door_right_2 (Variables|Default|GetEast_Door_Right))
  (bind _east_door_left_2 (Variables|Default|GetEast_Door_Left))
  (bind _relativelocation (Variables|/Script/Engine.SceneComponent|GetRelativeLocation _east_door_right_2))
  (bind _relativelocation_2 (Variables|/Script/Engine.SceneComponent|GetRelativeLocation _east_door_right))
  (bind _relativelocation_3 (Variables|/Script/Engine.SceneComponent|GetRelativeLocation _east_door_left_2))
  (bind _relativelocation_4 (Variables|/Script/Engine.SceneComponent|GetRelativeLocation _east_door_left))
  (Utilities|Casting|CastToTwinStickPawn OtherActor)
  (Variables|Default|SetopenEastDoor false)
  (if (Variables|Default|GetopenEastDoor)
    (Variables|Default|SeteastRelativeLeftDoorLocationY (- (.x _relativelocation_3) (Variables|Default|GetTILE_SIZE)))
    (Variables|Default|SeteastLeftOpenDoorPosition (Math|Vector|MakeVector (Variables|Default|GeteastRelativeLeftDoorLocationY) (.y _relativelocation_3) (.z _relativelocation_3)))
    (Variables|Default|SeteastRelativeRightDoorLocationY (+ (Variables|Default|GetTILE_SIZE) (.x _relativelocation)))
    (Variables|Default|SeteastRightOpenDoorPosition (Math|Vector|MakeVector (Variables|Default|GeteastRelativeRightDoorLocationY) (.y _relativelocation) (.z _relativelocation)))
    (bind _opendoor (Timeline|Timeline_2 PlayFromStart)
      (:Update
        (Transformation|SetRelativeLocation (Variables|Default|GetEast_Door_Left) (Math|Vector|Lerp(Vector) (Variables|/Script/Engine.SceneComponent|GetRelativeLocation (Variables|Default|GetEast_Door_Left)) (Variables|Default|GeteastLeftOpenDoorPosition) _opendoor) false false)
        (Transformation|SetRelativeLocation (Variables|Default|GetEast_Door_Right) (Math|Vector|Lerp(Vector) (Variables|/Script/Engine.SceneComponent|GetRelativeLocation (Variables|Default|GetEast_Door_Right)) (Variables|Default|GeteastRightOpenDoorPosition) _opendoor) false false)))
    (else
      (Utilities|FlowControl|Delay 1.0)
      (Variables|Default|SeteastRelativeLeftDoorLocationY (+ (Variables|Default|GetTILE_SIZE) (.x _relativelocation_4)))
      (Variables|Default|SeteastLeftClosedDoorPosition (Math|Vector|MakeVector (Variables|Default|GeteastRelativeLeftDoorLocationY) (.y _relativelocation_4) (.z _relativelocation_4)))
      (Variables|Default|SeteastRelativeRightDoorLocationY (- (.x _relativelocation_2) (Variables|Default|GetTILE_SIZE)))
      (Variables|Default|SeteastRightClosedDoorPosition (Math|Vector|MakeVector (Variables|Default|GeteastRelativeRightDoorLocationY) (.y _relativelocation_2) (.z _relativelocation_2)))
      (bind _closedoor (Timeline|Timeline_3 PlayFromStart)
        (:Update
          (Transformation|SetRelativeLocation (Variables|Default|GetEast_Door_Left) (Math|Vector|Lerp(Vector) (Variables|/Script/Engine.SceneComponent|GetRelativeLocation (Variables|Default|GetEast_Door_Left)) (Variables|Default|GeteastLeftClosedDoorPosition) _closedoor) false false)
          (Transformation|SetRelativeLocation (Variables|Default|GetEast_Door_Right) (Math|Vector|Lerp(Vector) (Variables|/Script/Engine.SceneComponent|GetRelativeLocation (Variables|Default|GetEast_Door_Right)) (Variables|Default|GeteastRightClosedDoorPosition) _closedoor) false false))))))

(event OnComponentBeginOverlap(SouthDoorController)
  (params (OverlappedComponent :type Primitive%20Component%20Object%20Reference) (OtherActor :type Actor%20Object%20Reference) (OtherComp :type Primitive%20Component%20Object%20Reference) (OtherBodyIndex :type Integer) (bFromSweep :type Boolean) (SweepResult :type Hit%20Result%20Structure%20%28by%20ref%29))
  (bind _south_door_right (Variables|Default|GetSouth_Door_Right))
  (bind _south_door_right_2 (Variables|Default|GetSouth_Door_Right))
  (bind _south_door_left (Variables|Default|GetSouth_Door_Left))
  (bind _south_door_left_2 (Variables|Default|GetSouth_Door_Left))
  (bind _relativelocation (Variables|/Script/Engine.SceneComponent|GetRelativeLocation _south_door_right_2))
  (bind _relativelocation_2 (Variables|/Script/Engine.SceneComponent|GetRelativeLocation _south_door_right))
  (bind _relativelocation_3 (Variables|/Script/Engine.SceneComponent|GetRelativeLocation _south_door_left))
  (bind _relativelocation_4 (Variables|/Script/Engine.SceneComponent|GetRelativeLocation _south_door_left_2))
  (Utilities|Casting|CastToTwinStickPawn OtherActor)
  (Variables|Default|SetopenSouthDoor true)
  (if (Variables|Default|GetopenSouthDoor)
    (Variables|Default|SetsouthRelativeLeftDoorLocationX (- (.x _relativelocation_3) (Variables|Default|GetTILE_SIZE)))
    (Variables|Default|SetsouthLeftOpenDoorPosition (Math|Vector|MakeVector (Variables|Default|GetsouthRelativeLeftDoorLocationX) (.y _relativelocation_3) (.z _relativelocation_3)))
    (Variables|Default|SetsouthRelativeRightDoorLocationX (+ (Variables|Default|GetTILE_SIZE) (.x _relativelocation)))
    (Variables|Default|SetsouthRightOpenDoorPosition (Math|Vector|MakeVector (Variables|Default|GetsouthRelativeRightDoorLocationX) (.y _relativelocation) (.z _relativelocation)))
    (bind _opendoor (Timeline|Timeline_4 PlayFromStart)
      (:Update
        (Transformation|SetRelativeLocation (Variables|Default|GetSouth_Door_Left) (Math|Vector|Lerp(Vector) (Variables|/Script/Engine.SceneComponent|GetRelativeLocation (Variables|Default|GetSouth_Door_Left)) (Variables|Default|GetsouthLeftOpenDoorPosition) _opendoor) false false)
        (Transformation|SetRelativeLocation (Variables|Default|GetSouth_Door_Right) (Math|Vector|Lerp(Vector) (Variables|/Script/Engine.SceneComponent|GetRelativeLocation (Variables|Default|GetSouth_Door_Right)) (Variables|Default|GetsouthRightOpenDoorPosition) _opendoor) false false)))
    (else
      (Utilities|FlowControl|Delay 1.0)
      (Variables|Default|SetsouthRelativeLeftDoorLocationX (+ (Variables|Default|GetTILE_SIZE) (.x _relativelocation_4)))
      (Variables|Default|SetsouthLeftClosedDoorPosition (Math|Vector|MakeVector (Variables|Default|GetsouthRelativeLeftDoorLocationX) (.y _relativelocation_4) (.z _relativelocation_4)))
      (Variables|Default|SetsouthRelativeRightDoorLocationX (- (.x _relativelocation_2) (Variables|Default|GetTILE_SIZE)))
      (Variables|Default|SetsouthRightClosedDoorPosition (Math|Vector|MakeVector (Variables|Default|GetsouthRelativeRightDoorLocationX) (.y _relativelocation_2) (.z _relativelocation_2)))
      (bind _closedoor (Timeline|Timeline_5 PlayFromStart)
        (:Update
          (Transformation|SetRelativeLocation (Variables|Default|GetSouth_Door_Left) (Math|Vector|Lerp(Vector) (Variables|/Script/Engine.SceneComponent|GetRelativeLocation (Variables|Default|GetSouth_Door_Left)) (Variables|Default|GetsouthLeftClosedDoorPosition) _closedoor) false false)
          (Transformation|SetRelativeLocation (Variables|Default|GetSouth_Door_Right) (Math|Vector|Lerp(Vector) (Variables|/Script/Engine.SceneComponent|GetRelativeLocation (Variables|Default|GetSouth_Door_Right)) (Variables|Default|GetsouthRightClosedDoorPosition) _closedoor) false false))))))

(event OnComponentEndOverlap(SouthDoorController)
  (params (OverlappedComponent :type Primitive%20Component%20Object%20Reference) (OtherActor :type Actor%20Object%20Reference) (OtherComp :type Primitive%20Component%20Object%20Reference) (OtherBodyIndex :type Integer))
  (bind _south_door_right (Variables|Default|GetSouth_Door_Right))
  (bind _south_door_right_2 (Variables|Default|GetSouth_Door_Right))
  (bind _south_door_left (Variables|Default|GetSouth_Door_Left))
  (bind _south_door_left_2 (Variables|Default|GetSouth_Door_Left))
  (bind _relativelocation (Variables|/Script/Engine.SceneComponent|GetRelativeLocation _south_door_right_2))
  (bind _relativelocation_2 (Variables|/Script/Engine.SceneComponent|GetRelativeLocation _south_door_right))
  (bind _relativelocation_3 (Variables|/Script/Engine.SceneComponent|GetRelativeLocation _south_door_left))
  (bind _relativelocation_4 (Variables|/Script/Engine.SceneComponent|GetRelativeLocation _south_door_left_2))
  (Utilities|Casting|CastToTwinStickPawn OtherActor)
  (Variables|Default|SetopenSouthDoor false)
  (if (Variables|Default|GetopenSouthDoor)
    (Variables|Default|SetsouthRelativeLeftDoorLocationX (- (.x _relativelocation_3) (Variables|Default|GetTILE_SIZE)))
    (Variables|Default|SetsouthLeftOpenDoorPosition (Math|Vector|MakeVector (Variables|Default|GetsouthRelativeLeftDoorLocationX) (.y _relativelocation_3) (.z _relativelocation_3)))
    (Variables|Default|SetsouthRelativeRightDoorLocationX (+ (Variables|Default|GetTILE_SIZE) (.x _relativelocation)))
    (Variables|Default|SetsouthRightOpenDoorPosition (Math|Vector|MakeVector (Variables|Default|GetsouthRelativeRightDoorLocationX) (.y _relativelocation) (.z _relativelocation)))
    (bind _opendoor (Timeline|Timeline_4 PlayFromStart)
      (:Update
        (Transformation|SetRelativeLocation (Variables|Default|GetSouth_Door_Left) (Math|Vector|Lerp(Vector) (Variables|/Script/Engine.SceneComponent|GetRelativeLocation (Variables|Default|GetSouth_Door_Left)) (Variables|Default|GetsouthLeftOpenDoorPosition) _opendoor) false false)
        (Transformation|SetRelativeLocation (Variables|Default|GetSouth_Door_Right) (Math|Vector|Lerp(Vector) (Variables|/Script/Engine.SceneComponent|GetRelativeLocation (Variables|Default|GetSouth_Door_Right)) (Variables|Default|GetsouthRightOpenDoorPosition) _opendoor) false false)))
    (else
      (Utilities|FlowControl|Delay 1.0)
      (Variables|Default|SetsouthRelativeLeftDoorLocationX (+ (Variables|Default|GetTILE_SIZE) (.x _relativelocation_4)))
      (Variables|Default|SetsouthLeftClosedDoorPosition (Math|Vector|MakeVector (Variables|Default|GetsouthRelativeLeftDoorLocationX) (.y _relativelocation_4) (.z _relativelocation_4)))
      (Variables|Default|SetsouthRelativeRightDoorLocationX (- (.x _relativelocation_2) (Variables|Default|GetTILE_SIZE)))
      (Variables|Default|SetsouthRightClosedDoorPosition (Math|Vector|MakeVector (Variables|Default|GetsouthRelativeRightDoorLocationX) (.y _relativelocation_2) (.z _relativelocation_2)))
      (bind _closedoor (Timeline|Timeline_5 PlayFromStart)
        (:Update
          (Transformation|SetRelativeLocation (Variables|Default|GetSouth_Door_Left) (Math|Vector|Lerp(Vector) (Variables|/Script/Engine.SceneComponent|GetRelativeLocation (Variables|Default|GetSouth_Door_Left)) (Variables|Default|GetsouthLeftClosedDoorPosition) _closedoor) false false)
          (Transformation|SetRelativeLocation (Variables|Default|GetSouth_Door_Right) (Math|Vector|Lerp(Vector) (Variables|/Script/Engine.SceneComponent|GetRelativeLocation (Variables|Default|GetSouth_Door_Right)) (Variables|Default|GetsouthRightClosedDoorPosition) _closedoor) false false))))))

(event OnComponentBeginOverlap(WestDoorController)
  (params (OverlappedComponent :type Primitive%20Component%20Object%20Reference) (OtherActor :type Actor%20Object%20Reference) (OtherComp :type Primitive%20Component%20Object%20Reference) (OtherBodyIndex :type Integer) (bFromSweep :type Boolean) (SweepResult :type Hit%20Result%20Structure%20%28by%20ref%29))
  (bind _west_door_left (Variables|Default|GetWest_Door_Left))
  (bind _west_door_right (Variables|Default|GetWest_Door_Right))
  (bind _west_door_right_2 (Variables|Default|GetWest_Door_Right))
  (bind _west_door_left_2 (Variables|Default|GetWest_Door_Left))
  (bind _relativelocation (Variables|/Script/Engine.SceneComponent|GetRelativeLocation _west_door_left_2))
  (bind _relativelocation_2 (Variables|/Script/Engine.SceneComponent|GetRelativeLocation _west_door_left))
  (bind _relativelocation_3 (Variables|/Script/Engine.SceneComponent|GetRelativeLocation _west_door_right))
  (bind _relativelocation_4 (Variables|/Script/Engine.SceneComponent|GetRelativeLocation _west_door_right_2))
  (Utilities|Casting|CastToTwinStickPawn OtherActor)
  (Variables|Default|SetopenWestDoor true)
  (if (Variables|Default|GetopenWestDoor)
    (Variables|Default|SetwestRelativeLeftDoorLocationY (- (.x _relativelocation_2) (Variables|Default|GetTILE_SIZE)))
    (Variables|Default|SetwestLeftOpenDoorPosition (Math|Vector|MakeVector (Variables|Default|GetwestRelativeLeftDoorLocationY) (.y _relativelocation_2) (.z _relativelocation_2)))
    (Variables|Default|SetwestRelativeRightDoorLocationY (+ (Variables|Default|GetTILE_SIZE) (.x _relativelocation_3)))
    (Variables|Default|SetwestRightOpenDoorPosition (Math|Vector|MakeVector (Variables|Default|GetwestRelativeRightDoorLocationY) (.y _relativelocation_3) (.z _relativelocation_3)))
    (bind _opendoor (Timeline|Timeline_6 PlayFromStart)
      (:Update
        (Transformation|SetRelativeLocation (Variables|Default|GetWest_Door_Left) (Math|Vector|Lerp(Vector) (Variables|/Script/Engine.SceneComponent|GetRelativeLocation (Variables|Default|GetWest_Door_Left)) (Variables|Default|GetwestLeftOpenDoorPosition) _opendoor) false false)
        (Transformation|SetRelativeLocation (Variables|Default|GetWest_Door_Right) (Math|Vector|Lerp(Vector) (Variables|/Script/Engine.SceneComponent|GetRelativeLocation (Variables|Default|GetWest_Door_Right)) (Variables|Default|GetwestRightOpenDoorPosition) _opendoor) false false)))
    (else
      (Utilities|FlowControl|Delay 1.0)
      (Variables|Default|SetwestRelativeLeftDoorLocationY (+ (Variables|Default|GetTILE_SIZE) (.x _relativelocation)))
      (Variables|Default|SetwestRightClosedDoorPosition (Math|Vector|MakeVector (Variables|Default|GetwestRelativeLeftDoorLocationY) (.y _relativelocation) (.z _relativelocation)))
      (Variables|Default|SetwestRelativeRightDoorLocationY (- (.x _relativelocation_4) (Variables|Default|GetTILE_SIZE)))
      (Variables|Default|SetwestRightClosedDoorPosition (Math|Vector|MakeVector (Variables|Default|GetwestRelativeRightDoorLocationY) (.y _relativelocation_4) (.z _relativelocation_4)))
      (bind _closedoor (Timeline|Timeline_7 PlayFromStart)
        (:Update
          (Transformation|SetRelativeLocation (Variables|Default|GetWest_Door_Left) (Math|Vector|Lerp(Vector) (Variables|/Script/Engine.SceneComponent|GetRelativeLocation (Variables|Default|GetWest_Door_Left)) (Variables|Default|GetwestLeftClosedDoorPosition) _closedoor) false false)
          (Transformation|SetRelativeLocation (Variables|Default|GetWest_Door_Right) (Math|Vector|Lerp(Vector) (Variables|/Script/Engine.SceneComponent|GetRelativeLocation (Variables|Default|GetWest_Door_Right)) (Variables|Default|GetwestRightClosedDoorPosition) _closedoor) false false))))))

(event OnComponentEndOverlap(WestDoorController)
  (params (OverlappedComponent :type Primitive%20Component%20Object%20Reference) (OtherActor :type Actor%20Object%20Reference) (OtherComp :type Primitive%20Component%20Object%20Reference) (OtherBodyIndex :type Integer))
  (bind _west_door_left (Variables|Default|GetWest_Door_Left))
  (bind _west_door_right (Variables|Default|GetWest_Door_Right))
  (bind _west_door_right_2 (Variables|Default|GetWest_Door_Right))
  (bind _west_door_left_2 (Variables|Default|GetWest_Door_Left))
  (bind _relativelocation (Variables|/Script/Engine.SceneComponent|GetRelativeLocation _west_door_left_2))
  (bind _relativelocation_2 (Variables|/Script/Engine.SceneComponent|GetRelativeLocation _west_door_left))
  (bind _relativelocation_3 (Variables|/Script/Engine.SceneComponent|GetRelativeLocation _west_door_right))
  (bind _relativelocation_4 (Variables|/Script/Engine.SceneComponent|GetRelativeLocation _west_door_right_2))
  (Utilities|Casting|CastToTwinStickPawn OtherActor)
  (Variables|Default|SetopenWestDoor false)
  (if (Variables|Default|GetopenWestDoor)
    (Variables|Default|SetwestRelativeLeftDoorLocationY (- (.x _relativelocation_2) (Variables|Default|GetTILE_SIZE)))
    (Variables|Default|SetwestLeftOpenDoorPosition (Math|Vector|MakeVector (Variables|Default|GetwestRelativeLeftDoorLocationY) (.y _relativelocation_2) (.z _relativelocation_2)))
    (Variables|Default|SetwestRelativeRightDoorLocationY (+ (Variables|Default|GetTILE_SIZE) (.x _relativelocation_3)))
    (Variables|Default|SetwestRightOpenDoorPosition (Math|Vector|MakeVector (Variables|Default|GetwestRelativeRightDoorLocationY) (.y _relativelocation_3) (.z _relativelocation_3)))
    (bind _opendoor (Timeline|Timeline_6 PlayFromStart)
      (:Update
        (Transformation|SetRelativeLocation (Variables|Default|GetWest_Door_Left) (Math|Vector|Lerp(Vector) (Variables|/Script/Engine.SceneComponent|GetRelativeLocation (Variables|Default|GetWest_Door_Left)) (Variables|Default|GetwestLeftOpenDoorPosition) _opendoor) false false)
        (Transformation|SetRelativeLocation (Variables|Default|GetWest_Door_Right) (Math|Vector|Lerp(Vector) (Variables|/Script/Engine.SceneComponent|GetRelativeLocation (Variables|Default|GetWest_Door_Right)) (Variables|Default|GetwestRightOpenDoorPosition) _opendoor) false false)))
    (else
      (Utilities|FlowControl|Delay 1.0)
      (Variables|Default|SetwestRelativeLeftDoorLocationY (+ (Variables|Default|GetTILE_SIZE) (.x _relativelocation)))
      (Variables|Default|SetwestRightClosedDoorPosition (Math|Vector|MakeVector (Variables|Default|GetwestRelativeLeftDoorLocationY) (.y _relativelocation) (.z _relativelocation)))
      (Variables|Default|SetwestRelativeRightDoorLocationY (- (.x _relativelocation_4) (Variables|Default|GetTILE_SIZE)))
      (Variables|Default|SetwestRightClosedDoorPosition (Math|Vector|MakeVector (Variables|Default|GetwestRelativeRightDoorLocationY) (.y _relativelocation_4) (.z _relativelocation_4)))
      (bind _closedoor (Timeline|Timeline_7 PlayFromStart)
        (:Update
          (Transformation|SetRelativeLocation (Variables|Default|GetWest_Door_Left) (Math|Vector|Lerp(Vector) (Variables|/Script/Engine.SceneComponent|GetRelativeLocation (Variables|Default|GetWest_Door_Left)) (Variables|Default|GetwestLeftClosedDoorPosition) _closedoor) false false)
          (Transformation|SetRelativeLocation (Variables|Default|GetWest_Door_Right) (Math|Vector|Lerp(Vector) (Variables|/Script/Engine.SceneComponent|GetRelativeLocation (Variables|Default|GetWest_Door_Right)) (Variables|Default|GetwestRightClosedDoorPosition) _closedoor) false false))))))

(fn ConstructionScript)