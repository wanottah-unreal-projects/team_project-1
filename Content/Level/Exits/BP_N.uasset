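; North exit double door that slides open when the TwinStickPawn enters its trigger and closes after it leaves.
; Begin and end overlap on NorthDoorController set OpenNorthDoor and share one branch, with a one-second delay before closing.
; Each branch offsets both panels' current X by TILESIZE in opposite directions, rather than using stored rest positions.
; Separate open and close timelines lerp the panels from their current locations toward those targets.
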(event OnComponentBeginOverlap(NorthDoorController)
  (params (OverlappedComponent :type Primitive%20Component%20Object%20Reference) (OtherActor :type Actor%20Object%20Reference) (OtherComp :type Primitive%20Component%20Object%20Reference) (OtherBodyIndex :type Integer) (bFromSweep :type Boolean) (SweepResult :type Hit%20Result%20Structure%20%28by%20ref%29))
  (bind _north_door_right (Variables|Default|GetNorth_Door_Right))
  (bind _north_door_right_2 (Variables|Default|GetNorth_Door_Right))
  (bind _north_door_left (Variables|Default|GetNorth_Door_Left))
  (bind _north_door_left_2 (Variables|Default|GetNorth_Door_Left))
  (bind _relativelocation (Variables|/Script/Engine.SceneComponent|GetRelativeLocation _north_door_left_2))
  (bind _relativelocation_2 (Variables|/Script/Engine.SceneComponent|GetRelativeLocation _north_door_left))
  (bind _relativelocation_3 (Variables|/Script/Engine.SceneComponent|GetRelativeLocation _north_door_right_2))
  (bind _relativelocation_4 (Variables|/Script/Engine.SceneComponent|GetRelativeLocation _north_door_right))
  (Utilities|Casting|CastToTwinStickPawn OtherActor)
  (Variables|Default|SetopenNorthDoor true)
  (if (Variables|Default|GetopenNorthDoor)
    (Variables|Default|SetnorthRelativeLeftDoorLocationX (- (.x _relativelocation_2) (Variables|Default|GetTILE_SIZE)))
    (Variables|Default|SetnorthLeftOpenDoorPosition (Math|Vector|MakeVector (Variables|Default|GetnorthRelativeLeftDoorLocationX) (.y _relativelocation_2) (.z _relativelocation_2)))
    (Variables|Default|SetnorthRelativeRightDoorLocationX (+ (Variables|Default|GetTILE_SIZE) (.x _relativelocation_3)))
    (Variables|Default|SetnorthRightOpenDoorPosition (Math|Vector|MakeVector (Variables|Default|GetnorthRelativeRightDoorLocationX) (.y _relativelocation_3) (.z _relativelocation_3)))
    (bind _opendoor (Timeline|Timeline_2 PlayFromStart)
      (:Update
        (Transformation|SetRelativeLocation (Variables|Default|GetNorth_Door_Left) (Math|Vector|Lerp(Vector) (Variables|/Script/Engine.SceneComponent|GetRelativeLocation (Variables|Default|GetNorth_Door_Left)) (Variables|Default|GetnorthLeftOpenDoorPosition) _opendoor) false false)
        (Transformation|SetRelativeLocation (Variables|Default|GetNorth_Door_Right) (Math|Vector|Lerp(Vector) (Variables|/Script/Engine.SceneComponent|GetRelativeLocation (Variables|Default|GetNorth_Door_Right)) (Variables|Default|GetnorthRightOpenDoorPosition) _opendoor) false false)))
    (else
      (Utilities|FlowControl|Delay 1.0)
      (Variables|Default|SetnorthRelativeLeftDoorLocationX (+ (Variables|Default|GetTILE_SIZE) (.x _relativelocation)))
      (Variables|Default|SetnorthLeftClosedDoorPosition (Math|Vector|MakeVector (Variables|Default|GetnorthRelativeLeftDoorLocationX) (.y _relativelocation) (.z _relativelocation)))
      (Variables|Default|SetnorthRelativeRightDoorLocationX (- (.x _relativelocation_4) (Variables|Default|GetTILE_SIZE)))
      (Variables|Default|SetnorthRightClosedDoorPosition (Math|Vector|MakeVector (Variables|Default|GetnorthRelativeRightDoorLocationX) (.y _relativelocation_4) (.z _relativelocation_4)))
      (bind _closedoor (Timeline|Timeline_3 PlayFromStart)
        (:Update
          (Transformation|SetRelativeLocation (Variables|Default|GetNorth_Door_Left) (Math|Vector|Lerp(Vector) (Variables|/Script/Engine.SceneComponent|GetRelativeLocation (Variables|Default|GetNorth_Door_Left)) (Variables|Default|GetnorthLeftClosedDoorPosition) _closedoor) false false)
          (Transformation|SetRelativeLocation (Variables|Default|GetNorth_Door_Right) (Math|Vector|Lerp(Vector) (Variables|/Script/Engine.SceneComponent|GetRelativeLocation (Variables|Default|GetNorth_Door_Right)) (Variables|Default|GetnorthRightClosedDoorPosition) _closedoor) false false))))))

(event OnComponentEndOverlap(NorthDoorController)
  (params (OverlappedComponent :type Primitive%20Component%20Object%20Reference) (OtherActor :type Actor%20Object%20Reference) (OtherComp :type Primitive%20Component%20Object%20Reference) (OtherBodyIndex :type Integer))
  (bind _north_door_right (Variables|Default|GetNorth_Door_Right))
  (bind _north_door_right_2 (Variables|Default|GetNorth_Door_Right))
  (bind _north_door_left (Variables|Default|GetNorth_Door_Left))
  (bind _north_door_left_2 (Variables|Default|GetNorth_Door_Left))
  (bind _relativelocation (Variables|/Script/Engine.SceneComponent|GetRelativeLocation _north_door_left_2))
  (bind _relativelocation_2 (Variables|/Script/Engine.SceneComponent|GetRelativeLocation _north_door_left))
  (bind _relativelocation_3 (Variables|/Script/Engine.SceneComponent|GetRelativeLocation _north_door_right_2))
  (bind _relativelocation_4 (Variables|/Script/Engine.SceneComponent|GetRelativeLocation _north_door_right))
  (Utilities|Casting|CastToTwinStickPawn OtherActor)
  (Variables|Default|SetopenNorthDoor false)
  (if (Variables|Default|GetopenNorthDoor)
    (Variables|Default|SetnorthRelativeLeftDoorLocationX (- (.x _relativelocation_2) (Variables|Default|GetTILE_SIZE)))
    (Variables|Default|SetnorthLeftOpenDoorPosition (Math|Vector|MakeVector (Variables|Default|GetnorthRelativeLeftDoorLocationX) (.y _relativelocation_2) (.z _relativelocation_2)))
    (Variables|Default|SetnorthRelativeRightDoorLocationX (+ (Variables|Default|GetTILE_SIZE) (.x _relativelocation_3)))
    (Variables|Default|SetnorthRightOpenDoorPosition (Math|Vector|MakeVector (Variables|Default|GetnorthRelativeRightDoorLocationX) (.y _relativelocation_3) (.z _relativelocation_3)))
    (bind _opendoor (Timeline|Timeline_2 PlayFromStart)
      (:Update
        (Transformation|SetRelativeLocation (Variables|Default|GetNorth_Door_Left) (Math|Vector|Lerp(Vector) (Variables|/Script/Engine.SceneComponent|GetRelativeLocation (Variables|Default|GetNorth_Door_Left)) (Variables|Default|GetnorthLeftOpenDoorPosition) _opendoor) false false)
        (Transformation|SetRelativeLocation (Variables|Default|GetNorth_Door_Right) (Math|Vector|Lerp(Vector) (Variables|/Script/Engine.SceneComponent|GetRelativeLocation (Variables|Default|GetNorth_Door_Right)) (Variables|Default|GetnorthRightOpenDoorPosition) _opendoor) false false)))
    (else
      (Utilities|FlowControl|Delay 1.0)
      (Variables|Default|SetnorthRelativeLeftDoorLocationX (+ (Variables|Default|GetTILE_SIZE) (.x _relativelocation)))
      (Variables|Default|SetnorthLeftClosedDoorPosition (Math|Vector|MakeVector (Variables|Default|GetnorthRelativeLeftDoorLocationX) (.y _relativelocation) (.z _relativelocation)))
      (Variables|Default|SetnorthRelativeRightDoorLocationX (- (.x _relativelocation_4) (Variables|Default|GetTILE_SIZE)))
      (Variables|Default|SetnorthRightClosedDoorPosition (Math|Vector|MakeVector (Variables|Default|GetnorthRelativeRightDoorLocationX) (.y _relativelocation_4) (.z _relativelocation_4)))
      (bind _closedoor (Timeline|Timeline_3 PlayFromStart)
        (:Update
          (Transformation|SetRelativeLocation (Variables|Default|GetNorth_Door_Left) (Math|Vector|Lerp(Vector) (Variables|/Script/Engine.SceneComponent|GetRelativeLocation (Variables|Default|GetNorth_Door_Left)) (Variables|Default|GetnorthLeftClosedDoorPosition) _closedoor) false false)
          (Transformation|SetRelativeLocation (Variables|Default|GetNorth_Door_Right) (Math|Vector|Lerp(Vector) (Variables|/Script/Engine.SceneComponent|GetRelativeLocation (Variables|Default|GetNorth_Door_Right)) (Variables|Default|GetnorthRightClosedDoorPosition) _closedoor) false false))))))

(fn ConstructionScript)